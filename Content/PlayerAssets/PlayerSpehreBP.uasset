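; Player sphere Blueprint with a spring-arm camera, handling impact sounds, trigger reactions and the pause and death screens.
; Hits play a click at the ball, and the spring arm's collision test is enabled on BeginPlay.
; Overlaps match object-name prefixes to either detach the camera in place or set the gravity flags once.
; P or Escape pauses with a cached menu widget, while destruction pauses and shows the death screen.
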(event Custom|OnActorHit_Event
  (params (SelfActor :type Actor%20Object%20Reference) (OtherActor :type Actor%20Object%20Reference) (NormalImpulse :type Vector) (Hit :type Hit%20Result%20Structure%20%28by%20ref%29))
  (Audio|SpawnSoundatLocation "/Game/PlayerAssets/Click.Click" (Transformation|GetWorldLocation (Variables|Default|GetBall))))

(event EventBeginPlay
  (Variables|/Script/Engine.SpringArmComponent|SetbDoCollisionTest (Variables|Default|GetSpringArm) true))

(event EventActorBeginOverlap
  (params (OtherActor :type Actor%20Object%20Reference))
  (bind _output_get (Variables|Default|SetotherActor OtherActor))
  (if (Utilities|Enum|Equal(Enum) (Utilities|String|GetSubstring (Utilities|GetObjectName _output_get) 0 14) (Variables|Default|GetReleaseTriggerName))
    (Class|SceneComponent|DetachfromParent (Variables|Default|GetCamera) true true)
    (elif (not (Variables|Default|GetGravityActive))
      (if (Utilities|Enum|Equal(Enum) (Utilities|String|GetSubstring (Utilities|GetObjectName _output_get) 0 8) (Variables|Default|GetGrav%20En%20Name))
        (Variables|Default|SetAllowGravity true)
        (Variables|Default|SetGravityActive true)))))

(event EventTick
  (params (DeltaSeconds :type Float%20%28single-precision%29)))

(event EventDestroyed
  (Utilities|IsValid (Variables|Default|GetDeath%20Ref)
    (:Is%20Valid
      _)
    (:Is%20Not%20Valid
      (bind _returnvalue (UserInterface|CreateWidget "/Game/UI/Menu/DeathScreen.DeathScreen_C"))
      (Variables|Default|SetDeath%20Ref _returnvalue)))
  (Game|SetGamePaused true)
  (Variables|/Script/Engine.PlayerController|SetbShowMouseCursor (Game|GetPlayerController 0) true)
  (UserInterface|Viewport|AddtoViewport (Variables|Default|GetDeath%20Ref) 0))

(event Input|KeyboardEvents|Escape
  (params (Key :type Key%20Structure :default "AnyKey"))
  (:Pressed
    (Utilities|IsValid (Variables|Default|GetPause%20Menu%20Ref)
      (:Is%20Valid
        _)
      (:Is%20Not%20Valid
        (bind _returnvalue (UserInterface|CreateWidget "/Game/UI/Menu/PauseScreen.PauseScreen_C"))
        (Variables|Default|SetPause%20Menu%20Ref _returnvalue)))
    (Game|SetGamePaused true)
    (UserInterface|Viewport|AddtoViewport (Variables|Default|GetPause%20Menu%20Ref) 0)
    (Variables|/Script/Engine.PlayerController|SetbShowMouseCursor (Game|GetPlayerController 0) true)))

(event Input|KeyboardEvents|P
  (params (Key :type Key%20Structure :default "AnyKey"))
  (:Pressed
    (Utilities|IsValid (Variables|Default|GetPause%20Menu%20Ref)
      (:Is%20Valid
        _)
      (:Is%20Not%20Valid
        (bind _returnvalue (UserInterface|CreateWidget "/Game/UI/Menu/PauseScreen.PauseScreen_C"))
        (Variables|Default|SetPause%20Menu%20Ref _returnvalue)))
    (Game|SetGamePaused true)
    (UserInterface|Viewport|AddtoViewport (Variables|Default|GetPause%20Menu%20Ref) 0)
    (Variables|/Script/Engine.PlayerController|SetbShowMouseCursor (Game|GetPlayerController 0) true)))

(fn ConstructionScript)